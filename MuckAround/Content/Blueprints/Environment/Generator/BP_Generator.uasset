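; BP_Generator is an interactable, fuel-powered generator that toggles between Active and Deactive gameplay tag states on an instant interaction while fuel remains.
; State changes switch its point light and start looping timers that ramp head spin up or down, scaling loop sound volume and pitch with rotation rate.
; Switching on by interaction also starts a fuel-drain timer, which updates a progress-bar widget and sets Deactive when empty.
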(event `self.ReceiveBeginPlay`
  (bind _output_get (set `self.FuelIndicatorBar` (cast `/Game/UI/3D/WBP_ProgressBar` (`WidgetComponent.GetWidget` (`self.FuelIndicator`)) :!pure true)))
  (set `/Game/UI/3D/WBP_ProgressBar.Name` "Fuel" _output_get)
  (`/Game/UI/3D/WBP_ProgressBar.SetProgress` (`self.FuelIndicatorBar`) (/ (`self.Fuel`) 100.0)))

(event `self.EDITOR_UpdateTagState`
  (params (NewTag :type "GameplayTag Structure"))
  (bind _pointlight (`self.PointLight`))
  (`|SwitchGameplayTag` NewTag
    (:`State.Active`
      (`self.ChangeGeneratorActiveState` true :!label _label)
      (`SceneComponent.SetVisibility` _pointlight true false))
    (:`State.Deactive`
      (`self.ChangeGeneratorActiveState` false :!label _label_2)
      (`SceneComponent.SetVisibility` _pointlight false false))))

(event `self.ReceiveNewState`
  (params (PreviousTag :type "GameplayTag Structure") (NewTag :type "GameplayTag Structure"))
  (`|SwitchGameplayTag` NewTag
    (:`State.Active`
      (goto _label))
    (:`State.Deactive`
      (goto _label_2))))

(event `ChangeGeneratorActiveState`
  (params (NewState :type Boolean))
  (bind _output_get (set `self.IsActive` NewState))
  (if _output_get
    (bind _returnvalue (`KismetSystemLibrary.K2_SetTimerDelegate` (delegate `RotateHead`) 0.05 true))
    (else
      (`KismetSystemLibrary.K2_ClearAndInvalidateTimerHandle` _returnvalue)
      (bind _returnvalue_2 (`KismetSystemLibrary.K2_SetTimerDelegate` (delegate `StopHeadRotation`) 0.05 true)))))

(event `self.Sphere.OnComponentBeginOverlap`
  (params (OverlappedComponent :type "PrimitiveComponent Object Reference") (OtherActor :type "Actor Object Reference") (OtherComp :type "PrimitiveComponent Object Reference") (OtherBodyIndex :type Integer) (bFromSweep :type Boolean) (SweepResult :type "HitResult Structure (by ref)"))
  (cast `BaseCharacter` OtherActor))

(event `InteractionFinished`
  (bind _pointlight (`self.PointLight`))
  (if (> (`self.Fuel`) 0.0)
    (`|SwitchGameplayTag` (`self.CurrentState`)
      (:`State.Active`
        (`TaggableInterface.SetTag` (struct :`TagName` "State.Deactive"))
        (`self.ChangeGeneratorActiveState` false)
        (`SceneComponent.SetVisibility` _pointlight false false)
        (`KismetSystemLibrary.K2_ClearAndInvalidateTimerHandle` (stale `InteractionFinished` _returnvalue)))
      (:`State.Deactive`
        (`TaggableInterface.SetTag` (struct :`TagName` "State.Active"))
        (`self.ChangeGeneratorActiveState` true)
        (`SceneComponent.SetVisibility` _pointlight true false)
        (bind _returnvalue (`KismetSystemLibrary.K2_SetTimerDelegate` (delegate `ConsumeFuel`) 0.1 true))))))

(event `RotateHead`
  (bind _sw_generatorloop (`self.SW_GeneratorLoop`))
  (bind _head (`self.Head`))
  (bind _returnvalue (/ (`self.RotationRate`) 10.0))
  (if (< (`self.RotationRate`) 10.0)
    (set `self.RotationRate` (+ (`self.RotationRate`) 0.1))
    (`AudioComponent.SetVolumeMultiplier` _sw_generatorloop _returnvalue)
    (`AudioComponent.SetPitchMultiplier` _sw_generatorloop _returnvalue))
  (`SceneComponent.K2_SetRelativeRotation` _head (`KismetMathLibrary.ComposeRotators` (`SceneComponent.RelativeRotation` _head) (`KismetMathLibrary.MakeRotator` 0.0 0.0 (`self.RotationRate`))) false false))

(event `StopHeadRotation`
  (bind _sw_generatorloop (`self.SW_GeneratorLoop`))
  (bind _head (`self.Head`))
  (bind _returnvalue (/ (`self.RotationRate`) 10.0))
  (set `self.RotationRate` (- (`self.RotationRate`) 0.1))
  (`AudioComponent.SetVolumeMultiplier` _sw_generatorloop _returnvalue)
  (`AudioComponent.SetPitchMultiplier` _sw_generatorloop _returnvalue)
  (if (<= (`self.RotationRate`) 0.0)
    (`KismetSystemLibrary.K2_ClearAndInvalidateTimerHandle` (stale `ChangeGeneratorActiveState` _returnvalue_2))
    (else
      (`SceneComponent.K2_SetRelativeRotation` _head (`KismetMathLibrary.ComposeRotators` (`SceneComponent.RelativeRotation` _head) (`KismetMathLibrary.MakeRotator` 0.0 0.0 (`self.RotationRate`))) false false))))

(event `ConsumeFuel`
  (bind _output_get (set `self.Fuel` (- (`self.Fuel`) 0.5)))
  (`/Game/UI/3D/WBP_ProgressBar.SetProgress` (`self.FuelIndicatorBar`) (/ _output_get 100.0))
  (if (<= (`self.Fuel`) 0.0)
    (set `self.Fuel` 0.0)
    (`KismetSystemLibrary.K2_ClearAndInvalidateTimerHandle` (stale `InteractionFinished` _returnvalue))
    (`TaggableInterface.SetTag` (struct :`TagName` "State.Deactive"))))

(fn `GetDesiredInteraction`
  (returns (OutTag :type "GameplayTag Structure") (OutTime :type "Float (single-precision)"))
  (return (struct) 0.0))

(fn `SetInteractionState`
  (params (InTag :type "GameplayTag Structure") (HeldTime :type "Float (single-precision)") (Instigator :type "Object Object Reference"))
  (returns (ReturnValue :type Boolean))
  (`self.InteractionFinished`)
  (return false))

(fn `UserConstructionScript`)