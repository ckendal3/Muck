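; BP_Light is an interactable light that toggles between active and deactive gameplay-tag states after a held interaction.
; A hold reaching HoldTime flips the state tag via SetTag.
; Runtime and editor tag-change events both drive SetLightVisible, which toggles the PointLight and the Cube's dynamic-material emissive scale.
; The dynamic material is created on BeginPlay, and the Sphere overlap only casts to BaseCharacter without further action.
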(event `self.ReceiveBeginPlay`
  (bind _cube (`self.Cube`))
  (bind _returnvalue (`PrimitiveComponent.CreateDynamicMaterialInstance` _cube 0 (`PrimitiveComponent.GetMaterial` _cube 0) "None"))
  (set `self.DynamicMaterialInstance` _returnvalue))

(event `self.EDITOR_UpdateTagState`
  (params (NewTag :type "GameplayTag Structure"))
  (`|SwitchGameplayTag` NewTag
    (:`State.Active`
      (`self.SetLightVisible` true :!label _label))
    (:`State.Deactive`
      (`self.SetLightVisible` false :!label _label_2))))

(event `self.ReceiveNewState`
  (params (PreviousTag :type "GameplayTag Structure") (NewTag :type "GameplayTag Structure"))
  (`|SwitchGameplayTag` NewTag
    (:`State.Active`
      (goto _label))
    (:`State.Deactive`
      (goto _label_2))))

(event `self.Sphere.OnComponentBeginOverlap`
  (params (OverlappedComponent :type "PrimitiveComponent Object Reference") (OtherActor :type "Actor Object Reference") (OtherComp :type "PrimitiveComponent Object Reference") (OtherBodyIndex :type Integer) (bFromSweep :type Boolean) (SweepResult :type "HitResult Structure (by ref)"))
  (cast `BaseCharacter` OtherActor))

(event `InteractionFinished`
  (`|SwitchGameplayTag` (`self.CurrentState`)
    (:`State.Active`
      (`TaggableInterface.SetTag` (struct :`TagName` "State.Deactive")))
    (:`State.Deactive`
      (`TaggableInterface.SetTag` (struct :`TagName` "State.Active")))))

(fn `GetDesiredInteraction`
  (returns (OutTag :type "GameplayTag Structure") (OutTime :type "Float (single-precision)"))
  (return (struct :`TagName` "State.Interaction.Held") (`self.HoldTime`)))

(fn `SetInteractionState`
  (params (InTag :type "GameplayTag Structure") (HeldTime :type "Float (single-precision)") (Instigator :type "Object Object Reference"))
  (returns (ReturnValue :type Boolean))
  (bind _returnvalue (>= HeldTime (`self.HoldTime`)))
  (`|ExecutionSequence`
    (:`then_0`
      (if _returnvalue
        (`self.InteractionFinished`)))
    (:`then_1`
      (return _returnvalue))))

(fn `SetLightVisible`
  (params (bNewVisibility :type Boolean))
  (bind _dynamicmaterialinstance (`self.DynamicMaterialInstance`))
  (`SceneComponent.SetVisibility` (`self.PointLight`) bNewVisibility false)
  (if bNewVisibility
    (`MaterialInstanceDynamic.SetScalarParameterValue` _dynamicmaterialinstance "EmissiveScale" 2.0)
    (else
      (`MaterialInstanceDynamic.SetScalarParameterValue` _dynamicmaterialinstance "EmissiveScale" 0.0))))

(fn `UserConstructionScript`)