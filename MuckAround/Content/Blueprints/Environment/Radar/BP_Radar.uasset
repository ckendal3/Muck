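; BP_Radar is an environment actor that players toggle between active and inactive states through a held interaction.
; State tag changes, including editor updates, show or hide its point light to match.
; Once the hold time is reached, it flips the state tag and adds to the hunger energy resource on the character cached from the cast in the sphere overlap, rather than the interaction's instigator.
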(event `self.EDITOR_UpdateTagState`
  (params (NewTag :type "GameplayTag Structure"))
  (`|SwitchGameplayTag` NewTag
    (:`State.Active`
      (`self.SetLightVisible` true :!label _label))
    (:`State.Deactive`
      (`self.SetLightVisible` false :!label _label_2))))

(event `self.ReceiveNewState`
  (params (PreviousTag :type "GameplayTag Structure") (NewTag :type "GameplayTag Structure"))
  (`|SwitchGameplayTag` NewTag
    (:`State.Active`
      (goto _label))
    (:`State.Deactive`
      (goto _label_2))))

(event `self.Sphere.OnComponentBeginOverlap`
  (params (OverlappedComponent :type "PrimitiveComponent Object Reference") (OtherActor :type "Actor Object Reference") (OtherComp :type "PrimitiveComponent Object Reference") (OtherBodyIndex :type Integer) (bFromSweep :type Boolean) (SweepResult :type "HitResult Structure (by ref)"))
  (bind _asbase_character (cast `BaseCharacter` OtherActor)))

(event `InteractionFinished`
  (`|ExecutionSequence`
    (:`then_0`
      (`|SwitchGameplayTag` (`self.CurrentState`)
        (:`State.Active`
          (`TaggableInterface.SetTag` (struct :`TagName` "State.Deactive")))
        (:`State.Deactive`
          (`TaggableInterface.SetTag` (struct :`TagName` "State.Active")))))
    (:`then_1`
      (bind _asresource_tracker (cast `ResourceTracker` (`ActionComponent.GetAction` (`BaseCharacter.ActionComponent` (stale `self.Sphere.OnComponentBeginOverlap` _asbase_character)) (struct :`TagName` "Resource.Tracker"))))
      (`ResourceTracker.AddResource` _asresource_tracker (struct :`TagName` "Survival.Energy.Hunger") 5.0))))

(fn `GetDesiredInteraction`
  (returns (OutTag :type "GameplayTag Structure") (OutTime :type "Float (single-precision)"))
  (return (struct :`TagName` "State.Interaction.Held") (`self.HoldTime`)))

(fn `SetInteractionState`
  (params (InTag :type "GameplayTag Structure") (HeldTime :type "Float (single-precision)") (Instigator :type "Object Object Reference"))
  (returns (ReturnValue :type Boolean))
  (bind _returnvalue (>= HeldTime (`self.HoldTime`)))
  (`|ExecutionSequence`
    (:`then_0`
      (if _returnvalue
        (`self.InteractionFinished`)))
    (:`then_1`
      (return _returnvalue))))

(fn `SetLightVisible`
  (params (bNewVisibility :type Boolean))
  (`SceneComponent.SetVisibility` (`self.PointLight`) bNewVisibility false))

(fn `UserConstructionScript`)