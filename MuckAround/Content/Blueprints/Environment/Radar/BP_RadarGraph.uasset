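; BP_RadarGraph is a radar environment Blueprint that appears intended to build a mesh grid graph but is unfinished.
; BeginPlay calls UpdateMeshGrid, which has an empty body, and the construction script is also empty.
; A disconnected node chain would add an SM_RadarGraphGridPrism component with M_Radar_Master, with grid-style offset math fed by constant zeros, so it never runs.
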(event `self.ReceiveBeginPlay`
  (`self.UpdateMeshGrid`))

(event `UpdateMeshGrid`)

(fn `UserConstructionScript`)