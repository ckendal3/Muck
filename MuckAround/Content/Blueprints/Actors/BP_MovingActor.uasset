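; BP_MovingActor is an actor whose static mesh moves between a start and end transform, toggled when a BaseCharacter enters its sphere.
; Overlap flips a State.Active/State.Deactive gameplay tag, and the state event plays or reverses the Movement timeline to lerp the mesh transform.
; The construction script sets the timeline's play rate from Duration and snaps the mesh to the default state for editor preview.
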(event `self.EDITOR_UpdateTagState`
  (params (NewTag :type "GameplayTag Structure"))
  (`|SwitchGameplayTag` NewTag
    (:`State.Active`
      (`SceneComponent.K2_SetRelativeTransform` (`self.StaticMesh`) (`self.EndTransform`) false true))
    (:`State.Deactive`
      (`SceneComponent.K2_SetRelativeTransform` (`self.StaticMesh`) (`self.StartTransform`) false true))))

(event `self.ReceiveNewState`
  (params (PreviousTag :type "GameplayTag Structure") (NewTag :type "GameplayTag Structure"))
  (`|SwitchGameplayTag` NewTag
    (:`State.Active`
      (bind (_direction _alpha) (`Timeline|Movement` :!label _label)
        (:`Update`
          (`SceneComponent.K2_SetRelativeTransform` (`self.StaticMesh`) (`KismetMathLibrary.TLerp` (`self.StartTransform`) (`self.EndTransform`) _alpha) false false))))
    (:`State.Deactive`
      (goto _label :!via `Reverse`))))

(event `self.Sphere.OnComponentBeginOverlap`
  (params (OverlappedComponent :type "PrimitiveComponent Object Reference") (OtherActor :type "Actor Object Reference") (OtherComp :type "PrimitiveComponent Object Reference") (OtherBodyIndex :type Integer) (bFromSweep :type Boolean) (SweepResult :type "HitResult Structure (by ref)"))
  (cast `BaseCharacter` OtherActor)
  (`|SwitchGameplayTag` (`self.CurrentState`)
    (:`State.Active`
      (`TaggableInterface.SetTag` (struct :`TagName` "State.Deactive")))
    (:`State.Deactive`
      (`TaggableInterface.SetTag` (struct :`TagName` "State.Active")))))

(fn `UserConstructionScript`
  (`TimelineComponent.SetPlayRate` (`self.Movement`) (`KismetMathLibrary.SafeDivide` 1.0 (`self.Duration`)))
  (`self.EDITOR_UpdateTagState` (`self.DefaultState`)))