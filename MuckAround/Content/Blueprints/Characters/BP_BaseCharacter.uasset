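; Base character Blueprint that forwards player action input to the equippable currently held in its InventoryComponent.
; Left mouse press toggles the primary action and F press toggles the tertiary action.
; Right mouse toggles the secondary action on both press and release, so it behaves as a hold.
; The character contains no action logic of its own, leaving behavior to the equippable.
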(event `Key|LeftMouseButton`
  (params (Key :type "Key Structure"))
  (:`Pressed`
    (`EquippableItem.TogglePrimaryAction` (`InventoryComponent.CurrentEquippable` (`self.InventoryComponent`)))))

(event `Key|RightMouseButton`
  (params (Key :type "Key Structure"))
  (:`Pressed`
    (`EquippableItem.ToggleSecondaryAction` (`InventoryComponent.CurrentEquippable` (`self.InventoryComponent`)) :!label _label))
  (:`Released`
    (goto _label)))

(event `Key|F`
  (params (Key :type "Key Structure"))
  (:`Pressed`
    (`EquippableItem.ToggleTertiaryAction` (`InventoryComponent.CurrentEquippable` (`self.InventoryComponent`)))))

(fn `UserConstructionScript`)